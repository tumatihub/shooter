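; BaseEnemy is an enemy Blueprint for a twin-stick game that sets up its health bar and can drop pickups.
; On BeginPlay it links the health bar widget to itself and caches the game mode's wave stats and the player's hero.
; Drop spawns ammo by the per-weapon chance matching the hero's inventory weapon at index 2, plus a health pickup that is effectively guaranteed.
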(event EventBeginPlay
  (bind _asenemy_health_bar (Utilities|Casting|CastToEnemyHealthBar (UserInterface|GetUserWidgetObject (Variables|Default|GetHealthBar))))
  (Variables|/Game/Blueprints/UI/EnemyHealthBar.EnemyHealthBar_C|SetOwner _asenemy_health_bar self)
  (bind _astwin_stick_mode (Utilities|Casting|CastToTwinStickMode (Game|GetGameMode)))
  (Variables|Default|SetWaveStats (Variables|/Game/Blueprints/TwinStickMode.TwinStickMode_C|GetWaveStats _astwin_stick_mode))
  (bind _ashero_character (Utilities|Casting|CastToHeroCharacter (Game|GetPlayerCharacter 0)))
  (Variables|Default|SetHero _ashero_character))

(event Collision|EventActorBeginOverlap
  (params (OtherActor :type Actor%20Object%20Reference)))

(event EventTick
  (params (DeltaSeconds :type Float%20%28single-precision%29)))

(fn ConstructionScript)

(fn Drop
  (Utilities|FlowControl|Sequence
    (:then_0
      (for _array_element (.AmmoDropChances (Utilities|Struct|BreakWaveStats (Variables|Default|GetWaveStats)))
        (if (== (.WeaponClass (Utilities|Struct|BreakAmmoDropRate _array_element)) (Utilities|GetClass (Utilities|Array|Get(acopy) (Variables|/Game/Blueprints/HeroCharacter.HeroCharacter_C|GetInventoryWeapons (Variables|Default|GetHero)) 2)))
          (if (< (Math|Random|RandomFloat) (.Chance (Utilities|Struct|BreakAmmoDropRate _array_element)))
            (bind _returnvalue (Game|SpawnActorfromClass "/Game/Blueprints/Pickups/Ammo.Ammo_C" (Transformation|GetActorTransform) "Undefined" 0 0))
            (Variables|/Game/Blueprints/Pickups/Ammo.Ammo_C|SetQtd _returnvalue (.Qtd (Utilities|Struct|BreakAmmoDropRate _array_element)))))))
    (:then_1
      (if (< (Math|Random|RandomFloat) 1.0)
        (bind _returnvalue_2 (Game|SpawnActorfromClass "/Game/Blueprints/Pickups/Health.Health_C" (Transformation|GetActorTransform) "Undefined" 0 0))
        (Variables|/Game/Blueprints/Pickups/Health.Health_C|SetQtd _returnvalue_2 10)))))