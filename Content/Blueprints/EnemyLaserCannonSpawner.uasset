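; An enemy spawner actor that keeps a population of laser cannon enemies in the level up to a set maximum.
; On BeginPlay it starts a looping timer whose interval comes from an enemies-per-second rate.
; Each tick counts all existing laser cannons and, if below the cap, spawns an AI cannon at a random point inside its SpawnVolume box and prints a debug message.
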(event Custom|SpawnEnemy
  (bind _spawnvolume (Variables|Default|GetSpawnVolume))
  (bind _outactors (Actor|GetAllActorsOfClass "/Game/Blueprints/Enemies/EnemyLaserCannon.EnemyLaserCannon_C"))
  (if (< (Utilities|Array|Length _outactors) (Variables|Default|GetMaxEnemyCount))
    (AI|SpawnAIFromClass "/Game/Blueprints/Enemies/EnemyLaserCannon.EnemyLaserCannon_C" 0 (Math|Random|RandomPointinBoundingBox (Transformation|GetWorldLocation _spawnvolume) (Components|Box|GetScaledBoxExtent _spawnvolume)) "0, 0, 0" false)
    (Development|PrintString "Respawn Enemy LaserCannon")))

(event EventBeginPlay
  (Utilities|Time|SetTimerbyFunctionName 0 "SpawnEnemy" (/ 1.0 (Variables|Default|GetEnemiesPerSecond)) true))

(fn ConstructionScript)