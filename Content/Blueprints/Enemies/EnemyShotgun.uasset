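; Shotgun-wielding enemy character for a twin-stick game, which spawns an E_Shotgun on its GunSocket and maps Fire input to its trigger.
; While the hero overlaps it, a looping timer deals damage at its attack rate.
; On death it calls Drop, adds score, ignores pawn and dynamic collision, then destroys itself after a delay.
; TakeSoul gives the player its weapon class as a secondary, and construction tints two body materials.
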(event Custom|DamageTheHero
  (Default|AffectHealth (Variables|Default|GetHero_0) (Variables|Default|GetDamage)))

(event Collision|EventActorEndOverlap
  (params (OtherActor :type Actor%20Object%20Reference))
  (if (== OtherActor (Variables|Default|GetHero_0))
    (Utilities|Time|ClearTimerbyFunctionName 0 "DamageTheHero")))

(event EventAffectHealth
  (params (Delta :type Float%20%28single-precision%29))
  (bind _capsulecomponent (Variables|Default|GetCapsuleComponent))
  (Class|BaseCharacter|CalculateHealth Delta)
  (Development|PrintString (Utilities|String|ToString(Float) (Variables|Default|GetHealth)))
  (if (Variables|Default|GetisDead)
    (CallFunction|Drop)
    (bind _astwin_stick_mode (Utilities|Casting|CastToTwinStickMode (Game|GetGameMode)))
    (Default|IncrementScore _astwin_stick_mode (Variables|Default|GetDeathScore))
    (Collision|SetCollisionResponsetoChannel _capsulecomponent "ECC_WorldDynamic" "ECR_Ignore")
    (Collision|SetCollisionResponsetoChannel _capsulecomponent "ECC_Pawn" "ECR_Ignore")
    (Class|Pawn|DetachfromControllerPendingDestroy)
    (Utilities|FlowControl|Delay 3.0)
    (Actor|DestroyActor)))

(event EventTakeSoul
  (bind _ashero_character (Utilities|Casting|CastToHeroCharacter (Game|GetPlayerCharacter 0)))
  (Default|NewSecondaryWeapon _ashero_character (Variables|Default|GetEnemyWeaponClass)))

(event EventBeginPlay
  (bind _mesh (Variables|Character|GetMesh))
  (|CallParentFunction)
  (bind _returnvalue (Game|SpawnActorfromClass "/Game/Blueprints/Weapons/EnemyWeapons/E_Shotgun.E_Shotgun_C" (Transformation|GetWorldTransform _mesh) "Undefined" 0 0))
  (bind _output_get (Variables|Default|SetWeapon _returnvalue))
  (Transformation|AttachComponentToComponent _output_get _mesh "GunSocket" "SnapToTarget" "SnapToTarget" "SnapToTarget" true))

(event Collision|EventActorBeginOverlap
  (params (OtherActor :type Actor%20Object%20Reference))
  (bind _ashero_character (Utilities|Casting|CastToHeroCharacter OtherActor))
  (Variables|Default|SetHero_0 _ashero_character)
  (Utilities|Time|SetTimerbyFunctionName 0 "DamageTheHero" (/ 1.0 (Variables|Default|GetAttacksPerSecond)) true))

(event Input|ActionEvents|InputActionFire
  (params (Key :type Key%20Structure))
  (bind _weapon (Variables|Default|GetWeapon))
  (:Pressed
    (Default|PullTrigger _weapon))
  (:Released
    (Default|ReleaseTrigger _weapon)))

(fn ConstructionScript
  (bind _returnvalue (Rendering|Material|CreateDynamicMaterialInstance (Variables|Character|GetMesh) 0 0 :!class /Script/Engine.PrimitiveComponent))
  (bind _output_get (Variables|Default|SetDynaMat _returnvalue))
  (Rendering|Material|SetVectorParameterValue _output_get "BodyColor" (Variables|Default|GetEnemyColor) :!class /Script/Engine.MaterialInstanceDynamic)
  (bind _returnvalue_2 (Rendering|Material|CreateDynamicMaterialInstance (Variables|Character|GetMesh) 1 0 :!class /Script/Engine.PrimitiveComponent))
  (Rendering|Material|SetVectorParameterValue _returnvalue_2 "BodyColor" (Variables|Default|GetLogoColor) :!class /Script/Engine.MaterialInstanceDynamic))