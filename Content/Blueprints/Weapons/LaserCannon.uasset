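; LaserCannon is a hero weapon Blueprint that fires a timed laser after a delay, rooting the hero during the shot.
; PullTrigger locks the attached HeroCharacter's movement and rotation, then a timer spawns a LaserCannonProjectile at the spawn point.
; When the laser duration ends, EndLaser destroys it, restores control and allows weapon switching.
; Named timers drive the sequence, with the cooldown timer set at trigger pull and again at laser end.
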(event Custom|EndCoolDown
  (Variables|Default|SetCanUse true)
  (Development|PrintString "LaserCannon Reloaded"))

(event Custom|EnableMovement
  (bind _hero (Variables|Default|GetHero))
  (Variables|/Game/Blueprints/HeroCharacter.HeroCharacter_C|SetCanMove _hero true)
  (Variables|/Game/Blueprints/HeroCharacter.HeroCharacter_C|SetCanRotate _hero true))

(event Custom|EndLaser
  (Actor|DestroyActor (Variables|Default|GetLaser))
  (CallFunction|EnableMovement)
  (Utilities|Time|SetTimerbyFunctionName 0 "EndCoolDown" (Variables|Default|GetCoolDown))
  (Variables|/Game/Blueprints/HeroCharacter.HeroCharacter_C|SetCanChangeWeapon (Variables|Default|GetHero) true))

(event Custom|FireCannon
  (bind _returnvalue (Game|SpawnActorfromClass "/Game/Blueprints/Weapons/LaserCannonProjectile.LaserCannonProjectile_C" (Transformation|GetWorldTransform (Variables|Default|GetProjectileSpawnPoint)) "Undefined" 0 0))
  (Variables|Default|SetLaser _returnvalue)
  (Utilities|Time|SetTimerbyFunctionName 0 "EndLaser" (Variables|Default|GetLaserDuration)))

(event EventReleaseTrigger)

(event EventFire
  (bind _ashero_character (Utilities|Casting|CastToHeroCharacter (Actor|GetAttachParentActor)))
  (bind _output_get (Variables|Default|SetHero _ashero_character))
  (Variables|/Game/Blueprints/HeroCharacter.HeroCharacter_C|SetCanMove _output_get false)
  (Variables|/Game/Blueprints/HeroCharacter.HeroCharacter_C|SetCanRotate _output_get false)
  (Utilities|Time|SetTimerbyFunctionName 0 "FireCannon" (Variables|Default|GetTimerToShoot)))

(event EventBeginPlay)

(event EventPullTrigger
  (if (Variables|Default|GetCanUse)
    (CallFunction|Fire)
    (Variables|Default|SetCanUse false)
    (Utilities|Time|SetTimerbyFunctionName 0 "EndCoolDown" (Variables|Default|GetCoolDown))))

(fn ConstructionScript
  (|CallParentFunction))