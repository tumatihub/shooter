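; Twin-stick enemy spawner that releases a wave of AI enemies inside its spawn volume.
; SpawnWave stores the wave stats and starts a looping SpawnEnemy timer, using EnemiesPerSecond directly as the interval.
; Each tick spawns an EnemyCharacter at a random point in the box and passes it the wave stats.
; Once the count is reached, the uncleared timer calls StartCheckWaveClear on TwinStickMode every tick.
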(event Custom|SpawnEnemy
  (bind _spawnvolume (Variables|Default|GetSpawnVolume))
  (if (< (Variables|Default|GetSpawnedEnemies) (Variables|Default|GetMaxEnemyCount))
    (bind _returnvalue (AI|SpawnAIFromClass "/Game/Blueprints/Enemies/EnemyCharacter.EnemyCharacter_C" 0 (Math|Random|RandomPointinBoundingBox (Transformation|GetWorldLocation _spawnvolume) (Components|Box|GetScaledBoxExtent _spawnvolume)) "0, 0, 0" false))
    (Math|Integer|IncrementInt (Variables|Default|GetSpawnedEnemies)
      (:%20%20
        (bind _asenemy_character (Utilities|Casting|CastToEnemyCharacter _returnvalue))
        (Default|InitWaveStats _asenemy_character (Variables|Default|GetWaveStats))))
    (else
      (bind _astwin_stick_mode (Utilities|Casting|CastToTwinStickMode (Game|GetGameMode)))
      (Default|StartCheckWaveClear _astwin_stick_mode))))

(event Custom|SpawnWave
  (params (WaveStats :type Wave%20Stats%20Structure))
  (bind _output_get (Variables|Default|SetWaveStats WaveStats))
  (Variables|Default|SetSpawnedEnemies 0)
  (Variables|Default|SetMaxEnemyCount (.NumEnemies (Utilities|Struct|BreakWaveStats _output_get)))
  (Utilities|Time|SetTimerbyFunctionName 0 "SpawnEnemy" (.EnemiesPerSecond (Utilities|Struct|BreakWaveStats _output_get)) true))

(fn ConstructionScript)