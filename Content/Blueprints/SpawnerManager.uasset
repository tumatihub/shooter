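; SpawnerManager spawns enemy waves from the level's EnemySpawner actors and hands off to TwinStickMode for wave-clear checks.
; SpawnWave starts a looping timer, using EnemiesPerSecond as its interval, that spawns AI at random points in a random spawner's volume and passes them WaveStats.
; Enemy class comes from sequential chance rolls, defaulting to EnemyCharacter.
; The timer is never cleared here, so StartCheckWaveClear repeats once the count is reached.
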(event Custom|SpawnEnemy
  (bind _randomspawnvolume (Variables|Default|GetRandomSpawnVolume))
  (if (< (Variables|Default|GetSpawnedEnemies) (Variables|Default|GetMaxEnemyCount))
    (CallFunction|ChooseRandSpawner)
    (CallFunction|ChooseEnemyClass)
    (bind _returnvalue (AI|SpawnAIFromClass (Variables|Default|GetEnemyClassToSpawn) 0 (Math|Random|RandomPointinBoundingBox (Transformation|GetWorldLocation _randomspawnvolume) (Components|Box|GetScaledBoxExtent _randomspawnvolume)) "0, 0, 0" false))
    (Math|Integer|IncrementInt (Variables|Default|GetSpawnedEnemies)
      (:%20%20
        (bind _asenemy_character (Utilities|Casting|CastToEnemyCharacter _returnvalue))
        (Default|InitWaveStats _asenemy_character (Variables|Default|GetWaveStats))))
    (else
      (bind _astwin_stick_mode (Utilities|Casting|CastToTwinStickMode (Game|GetGameMode)))
      (Default|StartCheckWaveClear _astwin_stick_mode))))

(event Custom|SpawnWave
  (params (WaveStats :type Wave%20Stats%20Structure))
  (bind _output_get (Variables|Default|SetWaveStats WaveStats))
  (Variables|Default|SetSpawnedEnemies 0)
  (Variables|Default|SetMaxEnemyCount (.NumEnemies (Utilities|Struct|BreakWaveStats _output_get)))
  (Utilities|Time|SetTimerbyFunctionName 0 "SpawnEnemy" (.EnemiesPerSecond (Utilities|Struct|BreakWaveStats _output_get)) true))

(event Custom|ChooseRandSpawner
  (bind _spawners (Variables|Default|GetSpawners))
  (Variables|Default|SetRandomSpawnVolume (Variables|/Game/Blueprints/EnemySpawner.EnemySpawner_C|GetSpawnVolume (Utilities|Array|Get(acopy) _spawners (Math|Random|RandomIntegerinRange 0 (- (Utilities|Array|Length _spawners) 1))))))

(event Custom|ChooseEnemyClass
  (Variables|Default|SetEnemyChoosed false)
  (for _array_element (.EnemyChances (Utilities|Struct|BreakWaveStats (Variables|Default|GetWaveStats)))
    (if (not (Variables|Default|GetEnemyChoosed))
      (if (< (Math|Random|RandomFloat) (.Chance (Utilities|Struct|BreakEnemyChance _array_element)))
        (Variables|Default|SetEnemyClassToSpawn (.EnemyClass (Utilities|Struct|BreakEnemyChance _array_element)))
        (Variables|Default|SetEnemyChoosed true))))
  (if (not (Variables|Default|GetEnemyChoosed))
    (Variables|Default|SetEnemyClassToSpawn "/Game/Blueprints/Enemies/EnemyCharacter.EnemyCharacter_C")))

(event EventBeginPlay
  (bind _outactors (Actor|GetAllActorsOfClass "/Game/Blueprints/EnemySpawner.EnemySpawner_C"))
  (Variables|Default|SetSpawners _outactors))

(event Collision|EventActorBeginOverlap
  (params (OtherActor :type Actor%20Object%20Reference)))

(event EventTick
  (params (DeltaSeconds :type Float%20%28single-precision%29)))

(fn ConstructionScript)