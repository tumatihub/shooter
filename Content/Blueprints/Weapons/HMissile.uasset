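; HMissile is a hero weapon that launches an HMissileProjectile from its spawn point on trigger pull, gated by a cooldown.
; Fire casts the parent actor to HeroCharacter, briefly disables its movement with a timer and spawns the projectile.
; A second timer ends the cooldown, re-arming the weapon, printing a reload message and setting the hero's CanChangeWeapon flag to true.
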(event Custom|EndCoolDown
  (Variables|Default|SetCanUse true)
  (Development|PrintString "HMissile Reloaded")
  (Variables|/Game/Blueprints/HeroCharacter.HeroCharacter_C|SetCanChangeWeapon (Variables|Default|GetHero) true))

(event Custom|EnableMovement
  (Variables|/Game/Blueprints/HeroCharacter.HeroCharacter_C|SetCanMove (Variables|Default|GetHero) true))

(event EventReleaseTrigger)

(event EventFire
  (bind _ashero_character (Utilities|Casting|CastToHeroCharacter (Actor|GetAttachParentActor)))
  (bind _output_get (Variables|Default|SetHero _ashero_character))
  (Variables|/Game/Blueprints/HeroCharacter.HeroCharacter_C|SetCanMove _output_get false)
  (Utilities|Time|SetTimerbyFunctionName 0 "EnableMovement" 0.3)
  (Game|SpawnActorfromClass "/Game/Blueprints/Weapons/HMissileProjectile.HMissileProjectile_C" (Transformation|GetWorldTransform (Variables|Default|GetProjectileSpawnPoint)) "Undefined" 0 0))

(event EventBeginPlay)

(event EventPullTrigger
  (if (Variables|Default|GetCanUse)
    (CallFunction|Fire)
    (Variables|Default|SetCanUse false)
    (Utilities|Time|SetTimerbyFunctionName 0 "EndCoolDown" (Variables|Default|GetCoolDown))))

(fn ConstructionScript
  (|CallParentFunction))