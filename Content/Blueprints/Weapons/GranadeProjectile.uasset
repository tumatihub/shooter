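; Grenade projectile that launches forward with an impulse on spawn and explodes after a timed fuse.
; The explosion adds the hero base damage from TwinStickMode to its own damage and applies it to every BaseCharacter_BP pawn within the blast radius.
; The actor then destroys itself.
; A debug sphere shows the explosion range every tick.
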(event Custom|DebugExplosionRange
  (Rendering|Debug|DrawDebugSphere (Transformation|GetWorldLocation (Variables|Default|GetLaserMesh)) (Variables|Default|GetExplosionRange) 12 "(R=0.723958,G=0.006461,B=0.000000,A=1.000000)" 0.01 1.0))

(event Custom|Explode
  (bind _astwin_stick_mode (Utilities|Casting|CastToTwinStickMode (Game|GetGameMode)))
  (bind _baseherodmg (Default|GetHeroBaseDmg _astwin_stick_mode))
  (Variables|Default|SetTotalDmg (+ _baseherodmg (Variables|Default|GetDamage)))
  (bind _outactors (Collision|SphereOverlapActors (Transformation|GetWorldLocation (Variables|Default|GetLaserMesh)) (Variables|Default|GetExplosionRange) (Utilities|Array|MakeArray "ObjectTypeQuery3") 0))
  (for _array_element _outactors
    (bind _asbase_character_bp (Utilities|Casting|CastToBaseCharacter_BP _array_element)
      (:then
        (Class|IDamageable|AffectHealth(Message) _asbase_character_bp (Variables|Default|GetTotalDmg)))
      (:CastFailed
        (Development|PrintString "Hello"))))
  (Actor|DestroyActor))

(event EventTick
  (params (DeltaSeconds :type Float%20%28single-precision%29))
  (CallFunction|DebugExplosionRange))

(event EventBeginPlay
  (bind _projectilecollision (Variables|Default|GetProjectileCollision))
  (Physics|AddImpulse _projectilecollision (* (Math|Vector|GetForwardVector _projectilecollision) (Variables|Default|GetImpulse)) "None" true)
  (Utilities|Time|SetTimerbyFunctionName 0 "Explode" (Variables|Default|GetTimeToExplode)))

(fn ConstructionScript)