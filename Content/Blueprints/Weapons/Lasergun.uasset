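; Lasergun weapon Blueprint that fires LaserProjectile actors automatically while the trigger is held.
; PullTrigger, gated by a DoOnce, fires immediately and starts a looping Fire timer at the CoolDown interval, while ReleaseTrigger clears it and resets the gate.
; Each shot spawns at ProjectileSpawnPoint and sets CanChangeWeapon on the player's HeroCharacter.
; A trigger pull also clears CanUse until a one-shot cooldown timer restores it.
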(event Custom|EndCooldown
  (Variables|Default|SetCanUse true))

(event EventReleaseTrigger
  (Utilities|Time|ClearTimerbyFunctionName 0 "Fire")
  (Utilities|FlowControl|DoOnce false) ; enters at Reset
)

(event EventPullTrigger
  (Utilities|FlowControl|DoOnce false
    (:Completed
      (CallFunction|Fire)
      (Utilities|Time|SetTimerbyFunctionName 0 "Fire" (Variables|Default|GetCoolDown) true)
      (Variables|Default|SetCanUse false)
      (Utilities|Time|SetTimerbyFunctionName 0 "EndCooldown" (Variables|Default|GetCoolDown)))))

(event EventFire
  (Game|SpawnActorfromClass "/Game/Blueprints/Weapons/LaserProjectile.LaserProjectile_C" (Transformation|GetWorldTransform (Variables|Default|GetProjectileSpawnPoint)) "Undefined" 0 0)
  (bind _ashero_character (Utilities|Casting|CastToHeroCharacter (Game|GetPlayerCharacter 0)))
  (Variables|/Game/Blueprints/HeroCharacter.HeroCharacter_C|SetCanChangeWeapon _ashero_character true))

(fn ConstructionScript
  (|CallParentFunction))