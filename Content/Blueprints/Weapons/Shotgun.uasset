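; Shotgun weapon Blueprint that fires a projectile from each of three arrow spawn points when the trigger is pulled.
; Pulling the trigger while usable fires, then locks the weapon until a cooldown timer re-enables it and prints a reload message.
; Firing casts the attach parent actor to HeroCharacter and briefly disables the hero's movement, restoring it by timer.
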(event Custom|EndCoolDown
  (Variables|Default|SetCanUse true)
  (Development|PrintString "Shotgun Reloaded"))

(event Custom|EnableMovement
  (Variables|/Game/Blueprints/HeroCharacter.HeroCharacter_C|SetCanMove (Variables|Default|GetHero) true))

(event EventReleaseTrigger)

(event EventFire
  (bind _ashero_character (Utilities|Casting|CastToHeroCharacter (Actor|GetAttachParentActor)))
  (bind _output_get (Variables|Default|SetHero _ashero_character))
  (Variables|/Game/Blueprints/HeroCharacter.HeroCharacter_C|SetCanMove _output_get false)
  (Utilities|Time|SetTimerbyFunctionName 0 "EnableMovement" 0.3)
  (for _array_element (Variables|Default|GetSpawnPoints)
    (bind _asarrow_component (Utilities|Casting|CastToArrowComponent _array_element)
      (:then
        (Game|SpawnActorfromClass "/Game/Blueprints/Weapons/ShotgunProjectile.ShotgunProjectile_C" (Transformation|GetWorldTransform _asarrow_component) "Undefined" 0 0))
      (:CastFailed
        (Development|PrintString "Hello")))))

(event EventBeginPlay
  (Variables|Default|SetSpawnPoints (Utilities|Array|MakeArray (Variables|Default|GetProjectileSpawnPoint1) (Variables|Default|GetProjectileSpawnPoint2) (Variables|Default|GetProjectileSpawnPoint3))))

(event EventPullTrigger
  (if (Variables|Default|GetCanUse)
    (CallFunction|Fire)
    (Variables|Default|SetCanUse false)
    (Utilities|Time|SetTimerbyFunctionName 0 "EndCoolDown" (Variables|Default|GetCoolDown))))

(fn ConstructionScript
  (|CallParentFunction))