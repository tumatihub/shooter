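; Homing missile projectile for a twin-stick shooter that explodes on actor overlap to deal area damage.
; On BeginPlay it adds the game mode's hero base damage to its own.
; Until it locks a target, Tick sphere-searches for enemies and homes on the first result if alive.
; Any overlap damages enemies within explosion range through IDamageable, then destroys the missile, with optional debug shapes for ranges and targeting.
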(event Custom|DebugDetectionRange
  (if (Variables|Default|GetDebug)
    (Rendering|Debug|DrawDebugSphere (Transformation|GetWorldLocation (Variables|Default|GetLaserMesh)) (Variables|Default|GetTargetDetectionRange) 12 "(R=1.000000,G=0.037429,B=0.000000,A=1.000000)" 0.01 1.0)))

(event Custom|DebugExplosionArea
  (if (Variables|Default|GetDebug)
    (Rendering|Debug|DrawDebugSphere (Transformation|GetWorldLocation (Variables|Default|GetLaserMesh)) (Variables|Default|GetExplosionRange) 12 "(R=1.000000,G=0.037429,B=0.000000,A=1.000000)" 1.0 1.0)))

(event Custom|DebugTarget
  (if (Variables|Default|GetDebug)
    (if (!= (Variables|Default|GetTarget) 0)
      (Rendering|Debug|DrawDebugCapsule (Transformation|GetActorLocation) 5e+01 5e+01 "0, 0,0.000000" "(R=1.000000,G=0.717085,B=0.000000,A=1.000000)" 0.01 1.0))))

(event Collision|EventActorBeginOverlap
  (params (OtherActor :type Actor%20Object%20Reference))
  (CallFunction|DebugExplosionArea)
  (bind _outactors (Collision|SphereOverlapActors (Transformation|GetWorldLocation (Variables|Default|GetProjectileCollision)) (Variables|Default|GetExplosionRange) (Utilities|Array|MakeArray "ObjectTypeQuery3") "/Game/Blueprints/Enemies/BaseEnemy.BaseEnemy_C"))
  (for _array_element _outactors
    (Variables|Default|SetAffectedByExplosion _array_element)
    (if (Utilities|DoesObjectImplementInterface _array_element "/Game/Blueprints/iDamageable.iDamageable_C")
      (Class|IDamageable|AffectHealth(Message) (Variables|Default|GetAffectedByExplosion) (Variables|Default|GetTotalDmg))))
  (Actor|DestroyActor))

(event EventBeginPlay
  (bind _astwin_stick_mode (Utilities|Casting|CastToTwinStickMode (Game|GetGameMode)))
  (bind _baseherodmg (Default|GetHeroBaseDmg _astwin_stick_mode))
  (Variables|Default|SetTotalDmg (+ _baseherodmg (Variables|Default|GetDamage))))

(event EventTick
  (params (DeltaSeconds :type Float%20%28single-precision%29))
  (CallFunction|DebugDetectionRange)
  (CallFunction|DebugTarget)
  (if (== (Variables|Default|GetTarget) 0)
    (bind _outactors (Collision|SphereOverlapActors (Transformation|GetWorldLocation (Variables|Default|GetProjectileCollision)) (Variables|Default|GetTargetDetectionRange) (Utilities|Array|MakeArray "ObjectTypeQuery3") "/Game/Blueprints/Enemies/BaseEnemy.BaseEnemy_C"))
    (if (!= (Utilities|Array|Get(acopy) _outactors) 0)
      (bind _asbase_enemy (Utilities|Casting|CastToBaseEnemy (Utilities|Array|Get(acopy) _outactors)))
      (if (not (Variables|/Script/TwinStickShooter.BaseCharacter|GetisDead _asbase_enemy))
        (bind _output_get (Variables|Default|SetTarget _asbase_enemy))
        (Variables|/Script/Engine.ProjectileMovementComponent|SetHomingTargetComponent (Variables|Default|GetProjectileMovement) (Variables|/Script/Engine.Actor|GetRootComponent _output_get))))))

(fn ConstructionScript)